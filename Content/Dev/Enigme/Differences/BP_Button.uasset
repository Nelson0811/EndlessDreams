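; BP_Button is a puzzle button in the Differences enigma that opens a linked door once it and its linked buttons are all activated.
; ActivateButton sets the button active, then loops through ButtonRef and calls Open on DoorRef only if every referenced button is active.
; Interact is an empty stub, and nothing in the graph resets the active state.
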(event EventBeginPlay)

(event Collision|EventActorBeginOverlap
  (params (OtherActor :type Actor%20Object%20Reference)))

(event EventTick
  (params (DeltaSeconds :type Float%20%28single-precision%29)))

(event EventActivateButton
  (Variables|Default|SetValide true)
  (Variables|Default|SetActivate true)
  (for _array_element (Variables|Default|GetButtonRef)
    (if (not (Variables|BP_Button_C|GetActivate _array_element))
      (Variables|Default|SetValide false)))
  (if (Variables|Default|GetValide)
    (Default|Open (Variables|Default|GetDoorRef))))

(fn ConstructionScript)

(fn Interact
  (return 0))