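; Interactable box Blueprint that spends a player key to update a linked door.
; On ActivateButton, a player holding exactly one key triggers a DoOnce that decrements the key count and sets DoorNeedkey to true on the referenced door.
; Debug PrintString messages report success or a missing key.
; The Interact function and construction script are empty.
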(event EventActivateButton
  (bind _player_ref (Variables|Default|GetPlayer%20ref))
  (if (== (Variables|/Game/ThirdPerson/Blueprints/BP_ThirdPersonCharacter.BP_ThirdPersonCharacter_C|GetKey _player_ref) 1)
    (Utilities|FlowControl|DoOnce false
      (:Completed
        (Variables|/Game/ThirdPerson/Blueprints/BP_ThirdPersonCharacter.BP_ThirdPersonCharacter_C|SetKey _player_ref (- (Variables|/Game/ThirdPerson/Blueprints/BP_ThirdPersonCharacter.BP_ThirdPersonCharacter_C|GetKey _player_ref) 1))
        (Variables|/Game/Nelson/Bp/Door/Bp_Door.Bp_Door_C|SetDoorNeedkey? (Variables|Default|GetDoorREF) true)
        (Development|PrintString "Vous avez truc de porte" true true "(R=0.000000,G=1.000000,B=0.292889,A=1.000000)")))
    (else
      (Development|PrintString "Need Key" true true "(R=1.000000,G=0.233938,B=0.000000,A=1.000000)"))))

(fn ConstructionScript)

(fn Interact
  (return 0))