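; Drawer Blueprint that slides its drawer box mesh open and closed on alternate ActivateButton calls.
; BeginPlay caches the box's relative location as the rest position.
; A FlipFlop plays or reverses a Timeline, whose track value offsets the box along local Y from that position.
; The Interact function and construction script are empty.
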(event EventBeginPlay
  (Variables|Default|SetRelative%20Location (Variables|/Script/Engine.SceneComponent|GetRelativeLocation (Variables|Default|GetSM_DrawerBox))))

(event EventActivateButton
  (bind _relative_location (Variables|Default|GetRelative%20Location))
  (Utilities|FlowControl|FlipFlop
    (:A
      (bind _newtrack_0 (Timeline|Timeline Play)
        (:Update
          (Transformation|SetRelativeLocation (Variables|Default|GetSM_DrawerBox) (Math|Vector|MakeVector (.x _relative_location) (+ (.y _relative_location) _newtrack_0) (.z _relative_location)) false false))))
    (:B
      (Timeline|Timeline Reverse))))

(fn ConstructionScript)

(fn Interact
  (return 0))